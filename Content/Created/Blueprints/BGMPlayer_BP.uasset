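; BGMPlayer_BP is a Blueprint that plays background music and game-result sounds.
; BeginPlay spawns the BGM as a 2D sound.
; Tick polls SZHGameModeBase, spawning a zombie laugh on game over or a win sound on game clear.
; No guard limits this, so the result sound respawns every frame while its flag holds, and nothing stops the BGM.
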(event `self.ReceiveBeginPlay`
  (`GameplayStatics.SpawnSound2D` "/Game/Sound/BGM/PlayBGM.PlayBGM" 1.0 1.0 0.0 null))

(event `self.ReceiveTick`
  (params (DeltaSeconds :type "Float (single-precision)"))
  (bind _returnvalue (`GameplayStatics.GetGameMode`))
  (`/Engine/EditorBlueprintResources/StandardMacros.IsValid` _returnvalue
    (:`Is Valid`
      (bind _asszhgame_mode_base (cast `SZHGameModeBase` _returnvalue))
      (if (`SZHGameModeBase.is_GameOver` _asszhgame_mode_base)
        (`GameplayStatics.SpawnSound2D` "/Game/Sound/BGM/Defeat.Zombie_Female_Lough1" 1.0 1.0 0.0 null)
        (elif (`SZHGameModeBase.is_GameClear` _asszhgame_mode_base)
          (`GameplayStatics.SpawnSound2D` "/Game/Sound/BGM/Win.Win" 1.0 1.0 0.0 null))))))

(fn `UserConstructionScript`)